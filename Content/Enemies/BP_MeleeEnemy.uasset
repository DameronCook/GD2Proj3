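; Melee enemy Blueprint, animated with an orc hammer attack, that chases the player character from BeginPlay.
; ChasePlayer runs AI MoveTo toward the player, then on success triggers a melee attack and re-calls itself after a short delay.
; The loop has no failure branch, so a failed move ends the chase.
; Attack_Melee plays the attack montage, while the Attack override only passes through the parent's success and damage results.
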(event `self.ReceiveBeginPlay`
  (`parent.ReceiveBeginPlay`)
  (`self.ChasePlayer`))

(event `ChasePlayer`
  (`|AIMoveTo` self (0.0 0.0 0.0) (`GameplayStatics.GetPlayerCharacter` 0) 150.0
    (:`OnSuccess`
      (`self.Attack_Melee`)
      (`KismetSystemLibrary.Delay` 0.2)
      (`self.ChasePlayer`))))

(event `Attack_Melee`
  (`|PlayMontage` (`self.Mesh`) "/Game/Fantasy_Pack/Characters/Orc_Hummer/Animations/Anim_Orc_Hummer_Attack_1_Montage.Anim_Orc_Hummer_Attack_1_Montage"))

(fn `Attack`
  (returns (Success :type Boolean) (DamageAmount :type Integer))
  (bind (_success _damageamount) (`parent.Attack`))
  (return _success _damageamount))

(fn `UserConstructionScript`
  (`parent.UserConstructionScript`))