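; Base enemy character Blueprint holding health, attack damage, speed and attack range, with stub Attack and IsParried functions, presumably for child overrides.
; SetStats applies speed to walk movement; TakeDamage subtracts health.
; On lethal damage it decrements the wave controller's enemy total, possibly ending the wave, halts movement and montage, and sets a get-hit blackboard flag.
; A separate DeathScript event plays a sound, then destroys the dead enemy after a delay.
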(event `DeathScript`
  ;[0.004553 0.02718 0.15 0.5] DeathScript
  (bind _isdead (`self.isDead`))
  (if _isdead
    (`GameplayStatics.PlaySoundAtLocation` "/Engine/VREditor/Sounds/VR_teleport_Cue.VR_teleport_Cue" (`self.K2_GetActorLocation`) (struct) 1.0 1.0 0.0 null null null null)
    ;;[1 0 0 0.5] Add death anim here, adjust delay
    (`KismetSystemLibrary.Delay` 1.0)
    (`self.K2_DestroyActor`)))

(fn `Attack`
  (returns (Success :type Boolean) (DamageAmount :type Integer))
  (return false (`self.AttackDamage`)))

(fn `GetStats`
  (returns (Health :type Integer) (AttackDamage :type Integer) (Speed :type "Float (double-precision)") (AttackRange :type "Float (double-precision)"))
  (return (`self.Health`) (`self.AttackDamage`) (`self.Speed`) (`self.AttackRange`)))

(fn `isDead`
  (returns (isDead :type Boolean))
  (return (< (`self.Health`) 1)))

(fn `isParried`
  (returns (isParried :type Boolean))
  (return false))

(fn `SetStats`
  (params (Health :type Integer) (AttackDamage :type Integer) (Speed :type "Float (double-precision)") (AttackRange :type "Float (double-precision)"))
  (set `self.Health` Health)
  (set `self.AttackDamage` AttackDamage)
  (bind _output_get (set `self.Speed` Speed))
  (set `CharacterMovementComponent.MaxWalkSpeed` _output_get (`self.CharacterMovement`))
  (set `self.AttackRange` AttackRange))

(fn `TakeDamage`
  (params (Damage :type Integer))
  (returns (NewHealth :type Integer))
  (bind _wavecontrollerref (`self.WaveControllerRef`))
  (bind _enemy_total (`/Game/WaveSystem/BP_WaveController.Enemy Total` _wavecontrollerref))
  (bind _output_get (set `self.Health` (- (`self.Health`) Damage)))
  (bind _isdead (`self.isDead`))
  (if _isdead
    (`/Engine/EditorBlueprintResources/StandardMacros.DecrementInt` _enemy_total
      (:`  `
        (if (< _enemy_total 1)
          (`/Game/WaveSystem/BP_WaveController.End Wave` _wavecontrollerref))
        (`MovementComponent.StopMovementImmediately` (`self.CharacterMovement`))
        (`self.StopAnimMontage` null)
        (`BlackboardComponent.SetValueAsBool` (`AIBlueprintHelperLibrary.GetBlackboard` null) (`self.KN_GetHit`) true)))))

(fn `UserConstructionScript`)