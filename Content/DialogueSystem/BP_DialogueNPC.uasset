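; Dialogue NPC for a two-player game that talks to the wizard (player 0) or warrior (player 1) entering its talk radius.
; Talk reads DT_Dialogue rows by name, showing text on that player's widget and playing audio, then waits out the clip plus padding.
; "Branch" rows show two options and enable temporary input for that player; "None" ends and resets.
; Leaving the walk-off radius jumps to the "Exit" row.
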(event `self.ReceiveBeginPlay`
  (set `self.CurrentLine` (`self.FirstLine`)))

(event `self.TalkRadius.OnComponentBeginOverlap`
  (params (OverlappedComponent :type "PrimitiveComponent Object Reference") (OtherActor :type "Actor Object Reference") (OtherComp :type "PrimitiveComponent Object Reference") (OtherBodyIndex :type Integer) (bFromSweep :type Boolean) (SweepResult :type "HitResult Structure (by ref)"))
  (if (not (`self.BusyTalking`))
    (cast `/Game/Wizard/BP_WizardChar` OtherActor ; Left Side
      (:`then`
        (set `self.Talking Player Index` 0))
      (:`CastFailed`
        (cast `/Game/Warrior/BP_WarriorChar` OtherActor) ; Right Side
        (set `self.Talking Player Index` 1)))
    (bind _returnvalue (`|CreateWidget` "/Game/DialogueSystem/WBP_Dialogue.WBP_Dialogue_C" (`GameplayStatics.GetPlayerController` (`self.Talking Player Index`))))
    (set `self.DialogueWidget` _returnvalue)
    (`UserWidget.AddToPlayerScreen` (`self.DialogueWidget`) 0)
    (`self.Talk`)))

(event `Talk`
  (bind _dialoguewidget (`self.DialogueWidget`))
  ; Setting current dialogue variables from data table
  (bind _returnvalue (`|GetDataTableRow` "/Game/DialogueSystem/DT_Dialogue.DT_Dialogue" (`self.CurrentLine`))
    (:`then`
      (set `self.Out Row Dialogue` (break `/Game/DialogueSystem/F_Dialogue` _returnvalue))
      (set `self.Out Row Audio` (`.Audio_5_E6F625FB104B204413A2EFAC8C219372` (break `/Game/DialogueSystem/F_Dialogue` _returnvalue)))
      (set `self.Out Row Next Line` (`.NextLine_8_1F6C4A817C4D68B4278149B72D28056E` (break `/Game/DialogueSystem/F_Dialogue` _returnvalue)))
      (set `self.BusyTalking` true)
      (set `self.Out Row Option A` (`.OptionA_19_3D0CB3A4AB4D00EB1D633883AA7DD61A` (break `/Game/DialogueSystem/F_Dialogue` _returnvalue)))
      (set `self.Out Row Option B` (`.OptionB_20_A0C04811BF48485A24875B859989023B` (break `/Game/DialogueSystem/F_Dialogue` _returnvalue)))
      (set `self.Out Row Next Line A` (`.NextLineA_13_597D17101E4C0147741FBFBB66E8FEFC` (break `/Game/DialogueSystem/F_Dialogue` _returnvalue)))
      (set `self.Out Row Next Line B` (`.NextLineB_14_ADA8F20B9E407B0B8A2C61A047E70E70` (break `/Game/DialogueSystem/F_Dialogue` _returnvalue)))
      ; Set text and play sound
      (`TextBlock.SetText` (`/Game/DialogueSystem/WBP_Dialogue.DialogueBox` (`self.DialogueWidget`)) (`KismetTextLibrary.Conv_StringToText` (`self.Out Row Dialogue`)))
      (`GameplayStatics.PlaySoundAtLocation` (`self.Out Row Audio`) (`SceneComponent.K2_GetComponentLocation` (`self.DefaultSceneRoot`)) (struct) 1.0 1.0 0.0 null null null null)
      ; Padding between lines
      (bind _returnvalue_2 (message `AnimationDataModel.GetPlayLength` (`self.Out Row Audio`)))
      (`KismetSystemLibrary.Delay` (+ _returnvalue_2 2.0))
      ; Do branching dialogue
      (if (== (`self.Out Row Next Line`) "Branch")
        (`TextBlock.SetText` (`/Game/DialogueSystem/WBP_Dialogue.OptionA` _dialoguewidget) (`KismetTextLibrary.Conv_StringToText` (`KismetStringLibrary.Concat_StrStr` "A) " (`self.Out Row Option A`))))
        (`TextBlock.SetText` (`/Game/DialogueSystem/WBP_Dialogue.OptionB` _dialoguewidget) (`KismetTextLibrary.Conv_StringToText` (`KismetStringLibrary.Concat_StrStr` "B) " (`self.Out Row Option B`))))
        (`Widget.SetVisibility` (`/Game/DialogueSystem/WBP_Dialogue.OptionsBox` _dialoguewidget) "Visible")
        (`self.EnableInput` (`GameplayStatics.GetPlayerController` (`self.Talking Player Index`)))
        (else
          ; Check if theres another line. If not, stop talking
          (if (== (`self.Out Row Next Line`) "None") :!label _label
            (`Widget.RemoveFromParent` (`self.DialogueWidget`))
            (set `self.BusyTalking` false)
            (set `self.CurrentLine` (`self.FirstLine`))
            (else
              (set `self.CurrentLine` (`self.Out Row Next Line`))
              (`self.Talk`))))))))

(event `Key|Gamepad_FaceButton_Bottom`
  (params (Key :type "Key Structure"))
  ; Dialogue input (These inputs are temporary)
  (:`Pressed`
    (set `self.Out Row Next Line` (`self.Out Row Next Line A`) :!label _label_2)
    (`self.DisableInput` (`GameplayStatics.GetPlayerController` (`self.Talking Player Index`)) :!label _label_3)
    (`Widget.SetVisibility` (`/Game/DialogueSystem/WBP_Dialogue.OptionsBox` (`self.DialogueWidget`)) "Hidden")
    (goto _label)))

(event `self.WalkOffRadius.OnComponentEndOverlap`
  (params (OverlappedComponent :type "PrimitiveComponent Object Reference") (OtherActor :type "Actor Object Reference") (OtherComp :type "PrimitiveComponent Object Reference") (OtherBodyIndex :type Integer))
  ; Walk away / Exit dialogue
  (set `self.CurrentLine` "Exit")
  (`Widget.SetVisibility` (`/Game/DialogueSystem/WBP_Dialogue.OptionsBox` (`self.DialogueWidget`)) "Hidden")
  (`self.Talk`))

(event `Key|One`
  (params (Key :type "Key Structure"))
  ; Dialogue input (These inputs are temporary)
  (:`Pressed`
    (goto _label_2)))

(event `Key|Gamepad_FaceButton_Right`
  (params (Key :type "Key Structure"))
  ; Dialogue input (These inputs are temporary)
  (:`Pressed`
    (set `self.Out Row Next Line` (`self.Out Row Next Line B`) :!label _label_4)
    (goto _label_3)))

(event `Key|Two`
  (params (Key :type "Key Structure"))
  ; Dialogue input (These inputs are temporary)
  (:`Pressed`
    (goto _label_4)))

(fn `UserConstructionScript`)