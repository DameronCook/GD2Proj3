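; Lightning mine spell actor that damages enemies within its sphere when its mine-set dispatcher fires.
; BeginPlay binds the Set event to that dispatcher.
; Set spawns a Niagara effect at the mine and subtracts LightningDamage directly from the Health of each overlapping BP_EnemyParent.
; After a short delay, it destroys the effect and itself.
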(event `self.ReceiveBeginPlay`
  (add `self.MineSetDispatcher` (delegate `Set`)))

(event `Set`
  (bind _returnvalue (`NiagaraFunctionLibrary.SpawnSystemAtLocation` (`self.System Template`) (`self.K2_GetActorLocation`) (struct) (1.0 1.0 1.0) false))
  (for _array_element (`PrimitiveComponent.GetOverlappingActors` (`self.Sphere`) (`self.Class Filter`))
    (bind _asbp_enemy_parent (cast `/Game/Enemies/BP_EnemyParent` _array_element))
    (set `/Game/Enemies/BP_EnemyParent.Health` (- (`/Game/Enemies/BP_EnemyParent.Health` _asbp_enemy_parent) (`self.LightningDamage`)) _asbp_enemy_parent))
  (`KismetSystemLibrary.Delay` 3.0)
  (`ActorComponent.K2_DestroyComponent` _returnvalue)
  (`self.K2_DestroyActor`))

(fn `UserConstructionScript`)