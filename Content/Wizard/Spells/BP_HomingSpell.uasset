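; Homing spell projectile actor that, on BeginPlay, flies toward the nearest enemy location read from the player's wizard character.
; A timeline lerps it from its Start component's world location to that position, captured once rather than tracked, then destroys it.
; Sphere overlap stores the enemy hit, and a timeline event track subtracts the spell's damage from that enemy's Health.
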(event `self.ReceiveBeginPlay`
  (bind _asbp_wizard_char (cast `/Game/Wizard/BP_WizardChar` (`GameplayStatics.GetPlayerCharacter` 0)))
  (`self.Shoot` (`/Game/Wizard/BP_WizardChar.NearestEnemyLoc` _asbp_wizard_char)))

(event `Shoot`
  (params (ClosestEnemyLocation :type "Vector Structure"))
  (bind _as_bp_enemy_parent (`self.As BP Enemy Parent`))
  (bind (_direction _newtrack_0) (`Timeline|Timeline`)
    (:`Update`
      (`self.K2_SetActorLocation` (`KismetMathLibrary.VLerp` (`SceneComponent.K2_GetComponentLocation` (`self.start`)) ClosestEnemyLocation _newtrack_0)))
    (:`Finished`
      (`self.K2_DestroyActor`))
    (:`NewTrack_1`
      (set `/Game/Enemies/BP_EnemyParent.Health` (- (`/Game/Enemies/BP_EnemyParent.Health` _as_bp_enemy_parent) (`self.HomingSpellDamage`)) _as_bp_enemy_parent))))

(event `self.Sphere1.OnComponentBeginOverlap`
  (params (OverlappedComponent :type "PrimitiveComponent Object Reference") (OtherActor :type "Actor Object Reference") (OtherComp :type "PrimitiveComponent Object Reference") (OtherBodyIndex :type Integer) (bFromSweep :type Boolean) (SweepResult :type "HitResult Structure (by ref)"))
  (bind _asbp_enemy_parent (cast `/Game/Enemies/BP_EnemyParent` OtherActor))
  (set `self.As BP Enemy Parent` _asbp_enemy_parent))

(fn `UserConstructionScript`)