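; BP_WaveController runs enemy waves, loading each one's spawn list, frequency and two locations from DT_WaveData by the CurrentWave enum.
; It spawns listed enemies one by one after a delay at a randomly chosen location, giving each a controller reference.
; EnemyDied counts down the total, and at zero EndWave advances the enum and spawns BP_TalkToGod with a controller reference.
; OpenShop creates ability-select widgets for two local players.
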(event `self.ReceiveBeginPlay`
  (`self.Wave Start`))

(event `Wave Start`
  (bind _returnvalue (`|GetDataTableRow` "/Game/WaveSystem/DT_WaveData.DT_WaveData" (`KismetStringLibrary.Conv_StringToName` (`|GetEnumeratorNameAsString` (`self.CurrentWave`))))
    (:`then`
      (set `self.Spawn Freq` (`.SpawnFreq_9_9E67A262824838BBDFDFF383549947B8` (break `/Game/WaveSystem/S_WaveStruct` _returnvalue)))
      (bind _output_get (set `self.EnemySpawnList` (`.SpawnList_17_406256F03146731546A554A4FB7EDB16` (break `/Game/WaveSystem/S_WaveStruct` _returnvalue))))
      (bind _output_get_2 (set `self.Enemy Total` (`KismetArrayLibrary.Array_Length` _output_get)))
      (`KismetSystemLibrary.PrintString` (`KismetStringLibrary.Conv_IntToString` _output_get_2) true true (struct :`R` 1.0 :`G` 0.554674 :`A` 1.0) 4.0)
      (set `self.Spawn Location` (`.Location` (break `RigVMFunction_MathTransformTransformVector` (`.SpawnLocation_21_99135650EE4DBE3EBFC0348F2585ABE5` (break `/Game/WaveSystem/S_WaveStruct` _returnvalue)))))
      (set `self.Spawn Location 2` (`.Location` (break `RigVMFunction_MathTransformTransformVector` (`.SpawnLocation2_23_8E291DC53B44A395A99D6C9E48BAB182` (break `/Game/WaveSystem/S_WaveStruct` _returnvalue)))))
      (`KismetSystemLibrary.PrintString` (`|GetEnumeratorNameAsString` (`self.CurrentWave`)))
      (`self.Spawn Enemy`))))

(event `Spawn Enemy`
  (`KismetSystemLibrary.Delay` (`self.Spawn Freq`))
  (`KismetSystemLibrary.PrintString` "Spawning Enemy!")
  (if (`KismetMathLibrary.RandomBool`)
    (set `self.Chosen Spawn` (`self.Spawn Location`))
    (else
      (set `self.Chosen Spawn` (`self.Spawn Location 2`))))
  (bind _returnvalue (`|SpawnActorFromClass` (`|GetArrayItem` (`self.EnemySpawnList`)) (`KismetMathLibrary.MakeTransform` (`self.Chosen Spawn`)) "Undefined" "MultiplyWithRoot" null null))
  (bind _asbp_enemy_parent (cast `/Game/Enemies/BP_EnemyParent` _returnvalue)
    (:`then`
      (set `/Game/Enemies/BP_EnemyParent.WaveControllerRef` self _asbp_enemy_parent)
      (`KismetArrayLibrary.Array_Remove` (`self.EnemySpawnList`))
      (`KismetSystemLibrary.PrintString` (`KismetStringLibrary.Conv_IntToString` (`KismetArrayLibrary.Array_Length` (`self.EnemySpawnList`))))
      (if (`KismetSystemLibrary.IsValidClass` (`|GetArrayItem` (`self.EnemySpawnList`)))
        (`self.Spawn Enemy`)))
    (:`CastFailed`
      (`KismetSystemLibrary.PrintString` "CAST FAILED!!!!!" true true (struct :`R` 1.0 :`B` 0.032209 :`A` 1.0) 5.0))))

(event `End Wave`
  (`KismetSystemLibrary.PrintString` "THIS IS WORKING")
  (set `self.CurrentWave` (cast `/Game/WaveSystem/E_Waves` (+ (`KismetMathLibrary.Conv_ByteToInt` (`self.CurrentWave`)) 1)))
  (bind _returnvalue (`|SpawnActorFromClass` "/Game/DialogueSystem/BP_TalkToGod.BP_TalkToGod_C" (`KismetMathLibrary.MakeTransform` (-11640.0 9290.0 230.0)) "Undefined" "MultiplyWithRoot" null null))
  (set `/Game/DialogueSystem/BP_DialogueNPC.WaveController` self _returnvalue))

(event `Open Shop`
  (bind _returnvalue (`|CreateWidget` "/Game/UI/WBP_AbilitySelect.WBP_AbilitySelect_C" (`GameplayStatics.GetPlayerController` 0)))
  (`UserWidget.AddToPlayerScreen` _returnvalue 0)
  (bind _returnvalue_2 (`|CreateWidget` "/Game/UI/WBP_AbilitySelect.WBP_AbilitySelect_C" (`GameplayStatics.GetPlayerController` 1)))
  (`UserWidget.AddToPlayerScreen` _returnvalue_2 0))

(fn `EnemyDied`
  (bind _output_get (set `self.Enemy Total` (- (`self.Enemy Total`) 1)))
  (if (<= _output_get 0)
    (`self.End Wave`))
  (return))

(fn `UserConstructionScript`)